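; BP_PRUEBAINTERACTUAR is a test Blueprint that briefly shows a UI widget when its Pepe event fires.
; Pepe creates a WB_TEST widget for the first player controller, adds it to the viewport, then removes it after a five-second delay.
; A node that would offset the Cube component's relative location by Move is left unconnected and never runs.
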(event Custom|Pepe
  (bind _returnvalue (UserInterface|CreateWidget "/Game/WB_TEST.WB_TEST_C" (Game|GetPlayerController 0)))
  (bind _output_get (Variables|Default|SettESTWIDF _returnvalue))
  (UserInterface|Viewport|AddtoViewport _output_get 0)
  (Utilities|FlowControl|Delay 5.0)
  (Widget|RemovefromParent (Variables|Default|GettESTWIDF)))

(fn ConstructionScript)