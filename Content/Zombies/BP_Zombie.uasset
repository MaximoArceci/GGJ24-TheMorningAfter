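; Zombie enemy that chases the player character and deals damage at close range.
; On BeginPlay it caches the player, then FollowPlayer re-issues AI MoveTo on a short delay loop until within attack distance.
; AttackPlayer sphere-traces for pawns forward from AttackTrace with debug drawing, damages the hit actor, then resumes following after a delay.
; A missed trace leaves Attacking set and does not restart the loop.
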(event Custom|Follow%20Player
  ;[1 1 1] Sigue al player
  (if (>= (Transformation|GetDistanceTo (Variables|Default|GetChar%20Ref)) 1.5e+02)
    (AI|AIMoveTo self "0, 0, 0" (Variables|Default|GetChar%20Ref) 5.0 false
      (:then
        (Utilities|FlowControl|Delay 0.1)
        (CallFunction|FollowPlayer)))
    (else
      (CallFunction|AttackPlayer))))

(event Custom|AttackPlayer
  (bind _attacktrace (Variables|Default|GetAttackTrace))
  (bind _returnvalue (Transformation|GetWorldLocation _attacktrace))
  ;[1 1 1] Daño al player
  (if (not (Variables|Default|Getattacking))
    (Variables|Default|Setattacking true)
    (bind (_outhit _returnvalue_2) (Collision|SphereTraceForObjects _returnvalue (+ _returnvalue (* (Math|Vector|GetForwardVector (Transformation|GetWorldRotation _attacktrace)) 2e+02)) 5e+02 (Utilities|Array|MakeArray "ObjectTypeQuery3") false 0 "ForDuration"))
    (if _returnvalue_2
      (Variables|Default|Setattacking false)
      (Game|Damage|ApplyDamage (.HitActor (Collision|BreakHitResult _outhit)) 1e+01 0 0)
      (Utilities|FlowControl|Delay 1.0)
      (CallFunction|FollowPlayer))))

(event EventBeginPlay
  (bind _asbp_third_person_character (Utilities|Casting|CastToBP_ThirdPersonCharacter (Game|GetPlayerCharacter 0)))
  (Variables|Default|SetChar%20Ref _asbp_third_person_character)
  (CallFunction|FollowPlayer))

(fn ConstructionScript)